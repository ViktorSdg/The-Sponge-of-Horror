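; NPCCharacter is an NPC Blueprint with a simple HP-based damage and death handler.
; On AnyDamage, it subtracts the incoming damage from HP and destroys the actor when HP reaches zero or below.
; The subtraction and death check run only if HP is already below zero, so damage is ignored while HP is zero or positive.
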(event `self.ReceiveAnyDamage`
  (params (Damage :type "Float (single-precision)") (DamageType :type "DamageType Object Reference") (InstigatedBy :type "Controller Object Reference") (DamageCauser :type "Actor Object Reference"))
  ;[1 1 1] EnemyDamageLogic
  (set `self.Incoming Damage` Damage)
  (if (< (`self.HP`) 0.0)
    (set `self.HP` (- (`self.HP`) (`self.Incoming Damage`)))
    (if (<= (`self.HP`) 0.0)
      (`self.K2_DestroyActor`))))

(fn `UserConstructionScript`)